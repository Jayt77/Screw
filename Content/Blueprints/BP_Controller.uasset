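; BP_Controller is a controller for a turn-based card game that relays player actions and card reveals.
; On BeginPlay it casts and caches the GS_Screw game state.
; OWNING-prefixed events forward ability activations, with itself as the player, and turn endings to that game state.
; A reveal event passes card data and a duration straight to the given card.
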(event `self.ReceiveBeginPlay`
  (bind _asgs_screw (cast `/Game/Blueprints/GS_Screw` (`GameplayStatics.GetGameState`)))
  (set `self.GameState` _asgs_screw))

(event `OWNING OnAbilityActivated`
  (params (Ability :type "ECardAbility Enum" :default "None"))
  (`/Game/Blueprints/GS_Screw.OnAbilityActivated` (`self.GameState`) self Ability))

(event `OWNING OnTurnEnded`
  (`/Game/Blueprints/GS_Screw.OnTurnEnded` (`self.GameState`)))

(event `OWNING RevealCard`
  (params (Card :type "/Game/Blueprints/BP_Card Object Reference") (CardData :type "CardData Structure") (Duration :type "Float (double-precision)"))
  (`/Game/Blueprints/BP_Card.RevealCard` Card CardData Duration))

(fn `UserConstructionScript`)