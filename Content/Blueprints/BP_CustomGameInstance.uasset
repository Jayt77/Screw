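; Custom Game Instance that initializes game settings, applies upscaling and anti-aliasing choices, and handles Steam lobby joining and session travel.
; Upscaling and AA requests update the JSON settings file object, then apply it after a short retriggerable delay.
; When Steam is available, Init binds lobby events: invites auto-join asynchronously and broadcast the result.
; On game creation, non-owner lobby members switch to game-only input and open the host's Steam address after a delay.
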(event `/Game/EasyOptionsMenu/EasyGameUI/BPI_EGUI_GameInstanceInterface.SetAndApplyUpscalingMethods`
  (params (RequestedUpscalingMethod :type "/Game/EasyOptionsMenu/Datas/E_UpscalingMethods Enum" :default "NewEnumerator0") (RequestedAA_Method :type "/Game/EasyOptionsMenu/Datas/E_AntiAliasingMethods Enum" :default "NewEnumerator0"))
  ;[1 0.4745 0.4247 1 40] Upscaling & Anti Aliasing Handling
  (`KismetSystemLibrary.DelayUntilNextTick`)
  (bind _outjsonobject (`JsonBlueprintFunctionLibrary.FromFile` (`/Game/EasyOptionsMenu/EasyGameUI/BFL_EasyFunctionUtilities.GetSettingsFilePath`)))
  (`/Game/EasyOptionsMenu/EasyGameUI/BFL_EasyFunctionUtilities.SetAA AndUpscalingMethods` RequestedUpscalingMethod RequestedAA_Method _outjsonobject)
  (`KismetSystemLibrary.RetriggerableDelay` 0.2)
  (`/Game/EasyOptionsMenu/EasyGameUI/BFL_EasyFunctionUtilities.ApplyAA AndUpscalingMethod` _outjsonobject))

(event `self.ReceiveInit`
  (`parent.ReceiveInit`)
  (`|ExecutionSequence`
    (:`then_0`
      (`KismetSystemLibrary.Delay` 0.2)
      (`/Game/EasyOptionsMenu/EasyGameUI/BFL_EasyFunctionUtilities.InitGameInstanceSettings`))
    (:`then_1`
      (if (`SteamUtilities.IsSteamAvailable`)
        (add `SteamProMatchmaking.LobbyInvite` (`SteamProMatchmaking.GetSteamMatchmaking`) (delegate `OnLobbyInvite`))
        (add `SteamProMatchmaking.LobbyGameCreated` (`SteamProMatchmaking.GetSteamMatchmaking`) (delegate `OnLobbyGameCreated`))))))

(event `OnLobbyInvite`
  (params (Data :type "LobbyInviteData Structure (by ref)"))
  (bind _data (`SteamCoreProMatchmakingAsyncActionJoinLobby.JoinLobbyAsync` (`.SteamIDLobby` (break `LobbyInviteData` Data)))
    (:`OnCallback`
      (bind (_steamidlobby _blocked _chatroomenterresponse) (break `JoinLobbyData` _data))
      (`KismetSystemLibrary.PrintString` (`|GetEnumeratorNameAsString` _chatroomenterresponse) true true (struct :`R` 0.638429 :`B` 1.0 :`A` 1.0) 50.0)
      (`self.OnLobbyJoined` _steamidlobby))))

(event `OnLobbyGameCreated`
  (params (Data :type "LobbyGameCreated Structure (by ref)"))
  (bind (_steamidlobby _steamidgameserver) (break `LobbyGameCreated` Data))
  (bind _output (`self.IsInLobby` _steamidlobby))
  (if _output
    (bind _returnvalue (`SteamProMatchmaking.GetLobbyOwner` _steamidlobby))
    (if (not (`SteamUtilities.Equal` _returnvalue (`SteamProUser.GetSteamID_Pure`)))
      (`WidgetBlueprintLibrary.SetInputMode_GameOnly` (`GameplayStatics.GetPlayerController` 0))
      (`KismetSystemLibrary.Delay` 2.0)
      (`KismetSystemLibrary.ExecuteConsoleCommand` (`KismetStringLibrary.Concat_StrStr` "open steam." (`SteamUtilities.BreakSteamID` _steamidgameserver)) null))))

(fn `IsInLobby`
  (params (LobbyID :type "SteamID Structure"))
  (returns (Output :type Boolean))
  (bind _returnvalue (`SteamProMatchmaking.GetNumLobbyMembers` LobbyID))
  (for _index (range _returnvalue)
    (bind _returnvalue_2 (`SteamProMatchmaking.GetLobbyMemberByIndex` LobbyID _index))
    (if (`SteamUtilities.Equal` _returnvalue_2 (`SteamProUser.GetSteamID_Pure`))
      (return true))))