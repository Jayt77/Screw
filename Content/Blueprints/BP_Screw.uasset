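; BP_Screw is an interactable screw actor that reports player interactions to the game mode.
; Highlight toggles custom depth rendering on its static mesh, and CanInteract always returns true.
; Interact casts the game mode to GM_Screw and calls PlayerCalledScrew with the interacting player; its owner check has empty branches, so it has no effect.
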(event `/Game/Blueprints/BPI_Interaction.Highlight`
  (params (`On?` :type Boolean))
  (`PrimitiveComponent.SetRenderCustomDepth` (`self.StaticMesh`) `On?`))

(event `/Game/Blueprints/BPI_Interaction.Interact`
  (params (Player :type "Controller Object Reference"))
  (if (== Player (`self.GetOwner`))
    _
    (else
      _))
  (bind _asgm_screw (cast `/Game/Blueprints/GM_Screw` (`GameplayStatics.GetGameMode`)))
  (`/Game/Blueprints/GM_Screw.PlayerCalledScrew` _asgm_screw Player))

(fn `CanInteract`
  (returns (CanInteract :type Boolean))
  (return true))

(fn `UserConstructionScript`)