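; Pawn component that lets a player interact with cards and decks by looking at them.
; Each tick on the locally controlled pawn, a camera line trace stores the current hit.
; Interact selects a hit card unless it is in transition, or flags a deck interaction, then passes the player and selection through SERVERHandleAction to the level's BP_CardManager.
; A separate SERVERInteract event forwards an interact message to a given target.
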(event `self.ReceiveBeginPlay`
  (bind _asbp_pawn (cast `/Game/Blueprints/BP_Pawn` (`self.GetOwner`)))
  (set `self.Pawn` _asbp_pawn)
  (set `self.Controller` (`GameplayStatics.GetPlayerController` 0))
  (bind _returnvalue (`GameplayStatics.GetActorOfClass` "/Game/Blueprints/BP_CardManager.BP_CardManager_C"))
  (set `self.CardManager` _returnvalue))

(event `self.ReceiveTick`
  (params (DeltaSeconds :type "Float (single-precision)"))
  (if (`Pawn.IsLocallyControlled` (`self.Pawn`))
    (`self.LineTraceFromCam`)))

(event `SERVER Interact`
  (params (Target :type "Object Object Reference") (Player :type "Controller Object Reference"))
  (message `/Game/Blueprints/BPI_Interaction.Interact` Target Player))

(event `SERVER HandleAction`
  (params (Player :type "Controller Object Reference") (CurrentSelectedCard :type "/Game/Blueprints/BP_Card Object Reference") (`DeckInteract?` :type Boolean))
  (`/Game/Blueprints/BP_CardManager.HandleCardAction` (`self.CardManager`) Player CurrentSelectedCard `DeckInteract?`))

(fn `Interact`
  (bind (_bblockinghit _binitialoverlap _time _distance _location _impactpoint _normal _impactnormal _physmat _hitactor) (`GameplayStatics.BreakHitResult` (`self.CurrentHit`)))
  (if (`KismetSystemLibrary.DoesImplementInterface` _hitactor "/Game/Blueprints/BPI_Card.BPI_Card_C")
    (bind _asbp_card (cast `/Game/Blueprints/BP_Card` _hitactor))
    (if (not (`/Game/Blueprints/BP_Card.InTransition?` _asbp_card))
      (set `self.PreviousSelectedCard` (`self.CurrentSelectedCard`))
      (bind _output_get (set `self.CurrentSelectedCard` _asbp_card))
      (`self.SERVER HandleAction` (`self.Controller`) _output_get))
    (else
      (cast `/Game/Blueprints/BP_Deck` _hitactor)
      (`self.SERVER HandleAction` (`self.Controller`) (`self.CurrentSelectedCard`) true))))

(fn `LineTraceFromCam`
  (bind _camera (`/Game/Blueprints/BP_Pawn.Camera` (`self.Pawn`)))
  (bind _returnvalue (`SceneComponent.K2_GetComponentLocation` _camera))
  (bind _outhit (`KismetSystemLibrary.LineTraceSingle` _returnvalue (+ _returnvalue (* (`SceneComponent.GetForwardVector` _camera) (`self.InteractionDistance`))) "TraceTypeQuery1"))
  (set `self.CurrentHit` _outhit))