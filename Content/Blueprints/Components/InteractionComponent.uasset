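; Pawn component that lets a player select cards and play them on a deck by looking at them.
; Each tick a camera line trace stores the current hit, which Interact reads to toggle or switch the selected card through interface messages.
; Hitting a deck sends the selection through a server event to PlayCard, which, with authority, finds its hand index and passes it to CardManager.
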(event `self.ReceiveBeginPlay`
  (bind _asbp_pawn (cast `/Game/Blueprints/BP_Pawn` (`self.GetOwner`)))
  (set `self.Pawn` _asbp_pawn)
  (set `self.Controller` (`GameplayStatics.GetPlayerController` 0)))

(event `self.ReceiveTick`
  (params (DeltaSeconds :type "Float (single-precision)"))
  (`self.LineTraceFromCam`))

(event `SERVER Interact`
  (params (Target :type "Object Object Reference") (Player :type "Controller Object Reference"))
  (message `/Game/Blueprints/BPI_Interaction.Interact` Target Player))

(event `SERVER PlayCard`
  (params (Controller :type "Controller Object Reference") (Card :type "Card Object Reference (by ref)"))
  (`self.PlayCard` Controller Card))

(fn `Interact`
  (bind (_bblockinghit _binitialoverlap _time _distance _location _impactpoint _normal _impactnormal _physmat _hitactor) (`GameplayStatics.BreakHitResult` (`self.CurrentHit`)))
  (if (`KismetSystemLibrary.DoesImplementInterface` _hitactor "/Game/Blueprints/BPI_Card.BPI_Card_C")
    (if (== _hitactor (`self.CurrentSelectedCard`))
      (message `/Game/Blueprints/BPI_Card.Deselected` (`self.CurrentSelectedCard`))
      (set `self.CurrentSelectedCard` null)
      (else
        (message `/Game/Blueprints/BPI_Card.Deselected` (`self.CurrentSelectedCard`))
        (bind _asbp_card (cast `/Game/Blueprints/BP_Card` _hitactor))
        (bind _output_get (set `self.CurrentSelectedCard` _asbp_card))
        (message `/Game/Blueprints/BPI_Card.Selected` _output_get)))
    (else
      (cast `/Game/Blueprints/BP_Deck` _hitactor)
      (`self.SERVER PlayCard` (`self.Controller`) (`self.CurrentSelectedCard`)))))

(fn `LineTraceFromCam`
  (bind _camera (`/Game/Blueprints/BP_Pawn.Camera` (`self.Pawn`)))
  (bind _returnvalue (`SceneComponent.K2_GetComponentLocation` _camera))
  (bind _outhit (`KismetSystemLibrary.LineTraceSingle` :`Start` _returnvalue :`End` (+ _returnvalue (* (`SceneComponent.GetForwardVector` _camera) (`self.InteractionDistance`))) :`TraceChannel` "TraceTypeQuery1" :`DrawDebugType` "ForOneFrame"))
  (set `self.CurrentHit` _outhit))

(fn `PlayCard`
  (params (Controller :type "Controller Object Reference") (Card :type "Card Object Reference (by ref)"))
  (`/Engine/EditorBlueprintResources/ActorComponentMacros.Switch Has Authority`
    (:`Authority`
      (bind _returnvalue (`GameplayStatics.GetActorOfClass` "/Script/Screw.CardManager"))
      (`KismetSystemLibrary.PrintString` (`KismetSystemLibrary.GetDisplayName` (`self.Controller`)))
      (bind _returnvalue_2 (`CardManager.GetPlayerHand` _returnvalue Controller))
      (`CardManager.PlayCard` _returnvalue Controller (`KismetArrayLibrary.Array_Find` _returnvalue_2 Card)))))