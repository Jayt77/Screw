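; BP_Card is a playing card actor that can be selected, highlighted, moved and temporarily revealed.
; A dynamic material swaps between the hidden Skrew texture and the CardData face, while custom depth drives highlighting and selection shifts the card vertically.
; RevealCard lerps it to a target via a timeline and, given a nonzero duration, later returns and hides it.
; LerpCardTo can also destroy the card on authority shortly after arrival.
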(event `InitMat`
  (bind _returnvalue (`PrimitiveComponent.CreateDynamicMaterialInstance` (`self.StaticMesh`) 0 "/Game/Images/M_Card.M_Card" "None"))
  (bind _output_get (set `self.DynamicMat` _returnvalue))
  (`MaterialInstanceDynamic.SetTextureParameterValue` _output_get "Texture" "/Game/Images/skrew.skrew"))

(event `self.ReceiveBeginPlay`
  (`self.InitMat`))

(event `/Game/Blueprints/BPI_Card.Activate`)

(event `/Game/Blueprints/BPI_Card.Selected`
  (`self.K2_SetActorLocation` (+ (`self.K2_GetActorLocation`) (0.0 0.0 10.0))))

(event `/Game/Blueprints/BPI_Card.Deselected`
  (`self.K2_SetActorLocation` (+ (`self.K2_GetActorLocation`) (0.0 0.0 -10.0))))

(event `RevealCard`
  (params (CardData :type "CardData Structure") (EndTransform :type "Transform Structure") (Duration :type "Float (double-precision)"))
  (set `self.OriginalTransform` (`self.GetTransform`))
  (`self.LerpCardTo` EndTransform)
  (`/Engine/EditorBlueprintResources/StandardMacros.IsValid` (`self.DynamicMat`)
    (:`Is Valid`
      _)
    (:`Is Not Valid`
      (`self.InitMat`)))
  (`MaterialInstanceDynamic.SetTextureParameterValue` (`self.DynamicMat`) "Texture" (`.Texture` (break `CardData` CardData)))
  (if (!= Duration 0.0)
    (`KismetSystemLibrary.Delay` Duration)
    (`self.LerpCardTo` (`self.OriginalTransform`))
    (`self.HideCard`)
    (`KismetSystemLibrary.PrintString` "LERP + HIDE")))

(event `HideCard`
  (`MaterialInstanceDynamic.SetTextureParameterValue` (`self.DynamicMat`) "Texture" "/Game/Images/skrew.skrew")
  (set `self.DynamicMat` null))

(event `OWNING Hide`
  (`self.HideCard`))

(event `/Game/Blueprints/BPI_Interaction.Highlight`
  (params (`On?` :type Boolean))
  (`PrimitiveComponent.SetRenderCustomDepth` (`self.StaticMesh`) `On?`))

(event `LerpCardTo`
  (params (EndTransform :type "Transform Structure") (`DestroyOnFinish?` :type Boolean))
  (set `self.CardTransform` (`self.GetTransform`))
  (bind (_direction _float) (`Timeline|Timeline` :!via `PlayFromStart`)
    (:`Update`
      (`self.K2_SetActorTransform` (`KismetMathLibrary.TLerp` (`self.CardTransform`) EndTransform _float)))
    (:`Finished`
      (if `DestroyOnFinish?`
        (`/Engine/EditorBlueprintResources/ActorMacros.Switch Has Authority`
          (:`Authority`
            (`KismetSystemLibrary.Delay` 2.0)
            (`self.K2_DestroyActor`)))))))

(fn `UserConstructionScript`)