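; Server-side card manager for the Screw card game, running the deck, deal, turns and card actions.
; GameMode events drive the pre-round peek and turn cycle, where each player draws, then swaps or activates the card's ability.
; Hand changes adjust scores through GameMode, while controller, card and GameState calls handle reveals and movement on clients.
; The opponent-swap ability only ends the turn, as its swap logic is unwired.
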(event `OnPreRoundStarted`
  (`self.InitializeDeck`)
  (`self.ShuffleDeck`)
  (`self.DealCardsToPlayers`)
  (`/Game/Blueprints/GS_Screw.CLIENT HighlightOwnedCards` (`self.GameState`) true))

(event `OnGameStarted`
  (`self.AdvanceTurn`)
  (set `self.CurrentRoundPhase` "NewEnumerator1")
  (`/Game/Blueprints/GS_Screw.CLIENT HighlightOwnedCards` (`self.GameState`) false))

(event `self.ReceiveBeginPlay`
  (`parent.ReceiveBeginPlay`)
  (`|ExecutionSequence`
    (:`then_0`
      (bind _asgm_screw (cast `/Game/Blueprints/GM_Screw` (`GameplayStatics.GetGameMode`)))
      (bind _output_get (set `self.GameMode` _asgm_screw))
      (add `/Game/Blueprints/GM_Screw.OnPreRoundStarted` _output_get (delegate `OnPreRoundStarted`))
      (add `/Game/Blueprints/GM_Screw.OnTurnTimerEnded` _output_get (delegate `OnTurnEnded`))
      (add `/Game/Blueprints/GM_Screw.OnGameStarted` _output_get (delegate `OnGameStarted`)))
    (:`then_1`
      (bind _asgs_screw (cast `/Game/Blueprints/GS_Screw` (`GameplayStatics.GetGameState`)))
      (set `self.GameState` _asgs_screw))
    (:`then_2`
      (bind _returnvalue (`GameplayStatics.GetActorOfClass` "/Game/Blueprints/BP_Deck.BP_Deck_C"))
      (set `self.DeckTransform` (`/Game/Blueprints/BP_Deck.TopTransform` _returnvalue)))))

(event `OnTurnEnded`
  (`|ExecutionSequence`
    (:`then_0`
      (`/Engine/EditorBlueprintResources/StandardMacros.IsValid` (`self.GetLastDrawnCard`)
        (:`Is Valid`
          (`self.DiscardCard` (`self.CurrentTurnPlayer`) (`self.GetLastDrawnCard`)))))
    (:`then_1`
      (bind _asbp_controller (cast `/Game/Blueprints/BP_Controller` (`self.CurrentTurnPlayer`)))
      (`/Game/Blueprints/BP_Controller.OWNING OnTurnEnded` _asbp_controller))
    (:`then_2`
      (`BlueprintMapLibrary.Map_Remove` (`self.NewDrawnCard`) (`self.CurrentTurnPlayer`)))
    (:`then_3`
      (`self.AdvanceTurn`))))

(event `self.PlayCard`
  (params (Controller :type "Controller Object Reference") (CardIndex :type Integer))
  (`parent.PlayCard` Controller CardIndex)
  (`self.AdvanceTurn`))

(event `self.AdvanceTurn`
  (`KismetSystemLibrary.Delay` (`self.TurnDelay`))
  (`parent.AdvanceTurn`)
  (set `self.CurrentTurnPhase` "NewEnumerator0")
  (`/Game/Blueprints/GM_Screw.ResetCurrentTurnTimer` (`self.GameMode`))
  (bind _returnvalue (`self.GrantCardFromDeck` (`self.CurrentTurnPlayer`) (`self.DeckTransform`)))
  (`BlueprintMapLibrary.Map_Add` (`self.NewDrawnCard`) (`self.CurrentTurnPlayer`) _returnvalue)
  (bind _asbp_pawn (cast `/Game/Blueprints/BP_Pawn` (`Controller.K2_GetPawn` (`self.CurrentTurnPlayer`))))
  (bind _asbp_controller (cast `/Game/Blueprints/BP_Controller` (`self.CurrentTurnPlayer`)))
  (bind _asbp_card (cast `/Game/Blueprints/BP_Card` _returnvalue))
  (`KismetSystemLibrary.Delay` 1.0)
  (`/Game/Blueprints/BP_Controller.OWNING RevealCard` _asbp_controller _asbp_card (`Card.CardData` _returnvalue) 0.0)
  (`/Game/Blueprints/BP_Card.CLIENT CardTransition` _asbp_card (`SceneComponent.K2_GetComponentToWorld` (`/Game/Blueprints/BP_Pawn.CardDrawnPos` _asbp_pawn)) false 0.0))

(event `SwapCards`
  (params (Player :type "Controller Object Reference") (`Keep card` :type "Card Object Reference") (`Discard card` :type "Card Object Reference"))
  (`/Game/Blueprints/GS_Screw.OnCardSwapped` (`self.GameState`) `Keep card` `Discard card`)
  (`self.DiscardCard` Player `Discard card`)
  (bind _asbp_card (cast `/Game/Blueprints/BP_Card` `Keep card`))
  (`/Game/Blueprints/BP_Card.OWNING Hide` _asbp_card)
  (`BlueprintMapLibrary.Map_Remove` (`self.NewDrawnCard`) Player)
  (`self.OnTurnEnded`))

(event `SwapOpponentCard`
  (params (Player :type "Controller Object Reference") (MyCard :type "/Game/Blueprints/BP_Card Object Reference") (OpponentCard :type "/Game/Blueprints/BP_Card Object Reference"))
  (bind _carddata (`Card.CardData` OpponentCard))
  (bind _carddata_2 (`Card.CardData` MyCard))
  (bind _ascontroller (cast `Controller` (`self.GetOwner` OpponentCard) :!pure true))
  (`/Game/Blueprints/GS_Screw.CLIENT OpponentCardSwap` (`self.GameState`) OpponentCard MyCard)
  (bind _returnvalue (`self.GetPlayerHand` Player))
  (`KismetArrayLibrary.Array_Add` _returnvalue OpponentCard)
  (`KismetArrayLibrary.Array_RemoveItem` _returnvalue MyCard)
  (`self.AddCardScore` Player _carddata)
  (`self.RemoveCardScore` Player _carddata_2)
  (bind _returnvalue_2 (`self.GetPlayerHand` _ascontroller))
  (`KismetArrayLibrary.Array_RemoveItem` _returnvalue_2 OpponentCard)
  (`KismetArrayLibrary.Array_Add` _returnvalue_2 MyCard)
  (`self.AddCardScore` _ascontroller _carddata_2)
  (`self.RemoveCardScore` _ascontroller _carddata))

(event `DiscardCard`
  (params (Player :type "Controller Object Reference") (Card :type "Card Object Reference"))
  (`|ExecutionSequence`
    (:`then_0`
      (`self.RemoveCardScore` Player (`Card.CardData` Card)))
    (:`then_1`
      (bind _returnvalue (`self.GetPlayerHand` Player))
      (`KismetArrayLibrary.Array_RemoveItem` _returnvalue Card)
      (bind _asbp_card (cast `/Game/Blueprints/BP_Card` Card))
      (`/Game/Blueprints/GS_Screw.OnCardDestroyed` (`self.GameState`) _asbp_card (`self.DeckTransform`)))))

(event `ActivateCard`
  (params (Card :type "Card Object Reference"))
  (bind (_name _description _value _texture _ability) (break `CardData` (`Card.CardData` Card)))
  (`/Engine/EditorBlueprintResources/StandardMacros.IsValid` Card
    (:`Is Valid`
      (if (`|EnumEquality` _ability)
        (`self.OnTurnEnded`)
        (else
          (`|ExecutionSequence`
            (:`then_0`
              (set `self.CurrentTurnPhase` "NewEnumerator1"))
            (:`then_1`
              (bind _asbp_controller (cast `/Game/Blueprints/BP_Controller` (`self.CurrentTurnPlayer`)))
              (`/Game/Blueprints/BP_Controller.OWNING OnAbilityActivated` _asbp_controller _ability))))))))

(event `HandleCardAction`
  (params (Player :type "Controller Object Reference") (CurrentSelectedCard :type "/Game/Blueprints/BP_Card Object Reference") (`DeckInteract?` :type Boolean))
  (bind (_carddata_name _carddata_description _carddata_value _carddata_texture _carddata_ability) (break `CardData` (`Card.CardData` (`self.GetLastDrawnCard`))))
  (switch `/Game/Blueprints/Enums/E_RoundPhase` (`self.CurrentRoundPhase`)
    (:`NewEnumerator0`
      (if (not `DeckInteract?`)
        (bind _output (`self.PlayerOwnsCard` Player CurrentSelectedCard))
        (if (and _output (< (`BlueprintMapLibrary.Map_Find` (`self.NoRevealedCards`) Player) (`self.NoPreRoundReveals`)))
          (`self.RevealSelfOne` Player CurrentSelectedCard)
          (`BlueprintMapLibrary.Map_Add` (`self.NoRevealedCards`) Player (+ (`BlueprintMapLibrary.Map_Find` (`self.NoRevealedCards`) Player) 1)))))
    (:`NewEnumerator1`
      (bind _output_2 (`self.IsPlayersTurn` Player))
      (if _output_2
        (switch `/Game/Blueprints/Enums/E_TurnPhase` (`self.CurrentTurnPhase`)
          (:`NewEnumerator0`
            (if `DeckInteract?`
              (`self.ActivateCard` (`self.GetLastDrawnCard`))
              (else
                (bind _output_3 (`self.PlayerOwnsCard` (`self.CurrentTurnPlayer`) CurrentSelectedCard))
                (if (and _output_3 (`self.isValidCard` CurrentSelectedCard))
                  (`self.SwapCards` (`self.CurrentTurnPlayer`) (`self.GetLastDrawnCard`) CurrentSelectedCard)))))
          (:`NewEnumerator1`
            (if (`self.isValidCard` CurrentSelectedCard)
              (switch `ECardAbility` _carddata_ability
                (:`RevealOpponentOne`
                  (`self.RevealOpponentOne` CurrentSelectedCard))
                (:`RevealSelfOne`
                  (`self.RevealSelfOne` (`self.CurrentTurnPlayer`) CurrentSelectedCard))
                (:`SwapOneNoReveal`
                  _)
                (:`DiscardOneSelf`
                  (`self.DiscardOneSelf` CurrentSelectedCard)))
              (`self.OnTurnEnded`))))))))

(fn `AddCardScore`
  (params (Controller :type "Controller Object Reference") (`Card Data` :type "CardData Structure"))
  (`/Game/Blueprints/GM_Screw.AddPlayerScore` (`self.GameMode`) Controller (`.Value` (break `CardData` `Card Data`))))

(fn `DiscardOneSelf`
  (params (Card :type "Card Object Reference"))
  (bind _output (`self.PlayerOwnsCard` (`self.CurrentTurnPlayer`) Card))
  (if _output
    (`self.DiscardCard` (`self.CurrentTurnPlayer`) Card)))

(fn `GetLastDrawnCard`
  (returns (Card :type "Card Object Reference"))
  (return (`BlueprintMapLibrary.Map_Find` (`self.NewDrawnCard`) (`self.CurrentTurnPlayer`))))

(fn `IsPlayersTurn`
  (params (Controller :type "Controller Object Reference"))
  (returns (Output :type Boolean))
  (return (== Controller (`self.CurrentTurnPlayer`))))

(fn `isValidCard`
  (params (Card :type "Card Object Reference"))
  (returns (ReturnValue :type Boolean))
  (return (and (`KismetSystemLibrary.IsValid` Card) (!= (`self.GetLastDrawnCard`) Card))))

(fn `PlayerOwnsCard`
  (params (Player :type "Controller Object Reference") (Card :type "Card Object Reference"))
  (returns (Output :type Boolean))
  (return (== (`self.GetOwner` Card) Player)))

(fn `RemoveCardScore`
  (params (Player :type "Controller Object Reference (by ref)") (CardData :type "CardData Structure (by ref)"))
  (`/Game/Blueprints/GM_Screw.AddPlayerScore` (`self.GameMode`) Player (* (`.Value` (break `CardData` CardData)) -1)))

(fn `RevealOpponentOne`
  (params (Card :type "/Game/Blueprints/BP_Card Object Reference"))
  (bind _output (`self.PlayerOwnsCard` (`self.CurrentTurnPlayer`) Card))
  (if (not _output)
    (bind _asbp_controller (cast `/Game/Blueprints/BP_Controller` (`self.CurrentTurnPlayer`)))
    (bind _asbp_pawn (cast `/Game/Blueprints/BP_Pawn` (`Controller.K2_GetPawn` (`self.CurrentTurnPlayer`))))
    (`/Game/Blueprints/BP_Controller.OWNING RevealCard` _asbp_controller Card (`Card.CardData` Card) 2.0)
    (`/Game/Blueprints/BP_Card.CLIENT CardTransition` Card (`SceneComponent.K2_GetComponentToWorld` (`/Game/Blueprints/BP_Pawn.RevealCardPos` _asbp_pawn)) false 2.0)))

(fn `RevealSelfOne`
  (params (Player :type "Controller Object Reference") (Card :type "/Game/Blueprints/BP_Card Object Reference"))
  (bind _output (`self.PlayerOwnsCard` Player Card))
  (if _output
    (bind _asbp_controller (cast `/Game/Blueprints/BP_Controller` Player))
    (bind _asbp_pawn (cast `/Game/Blueprints/BP_Pawn` (`Controller.K2_GetPawn` Player)))
    (`/Game/Blueprints/BP_Controller.OWNING RevealCard` _asbp_controller Card (`Card.CardData` Card) 2.0)
    (`/Game/Blueprints/BP_Card.CLIENT CardTransition` Card (`SceneComponent.K2_GetComponentToWorld` (`/Game/Blueprints/BP_Pawn.RevealCardPos` _asbp_pawn)) false 2.0)))

(fn `SpawnCardAtLocation`
  (params (CardData :type "CardData Structure (by ref)") (Transform :type "Transform Structure (by ref)") (Controller :type "Controller Object Reference"))
  (returns (ReturnValue :type "Card Object Reference"))
  (bind _returnvalue (`parent.SpawnCardAtLocation` CardData Transform Controller))
  (`self.AddCardScore` Controller CardData)
  (return _returnvalue))

(fn `SwapOpponentOne`
  (params (MyCard :type "/Game/Blueprints/BP_Card Object Reference") (OpponentCard :type "/Game/Blueprints/BP_Card Object Reference"))
  (returns (`Successful?` :type Boolean))
  (if (`self.isValidCard` MyCard)
    (bind _output (`self.PlayerOwnsCard` (`self.CurrentTurnPlayer`) MyCard))
    (if _output
      (bind _output_2 (`self.PlayerOwnsCard` (`self.CurrentTurnPlayer`) OpponentCard))
      (if (not _output_2)
        (`self.SwapOpponentCard` (`self.CurrentTurnPlayer`) OpponentCard OpponentCard)
        (return true)))))

(fn `UserConstructionScript`)