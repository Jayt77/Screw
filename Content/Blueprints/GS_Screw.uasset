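; GS_Screw is the game state for the Screw card game, handling local visual feedback for turns, abilities and card moves.
; Activated abilities switch the local BP_Pawn's view or highlight cards, splitting own from opponent cards by comparing owner to player controller 0.
; Turn end clears highlights and resets the view.
; Card destroy and swap events animate BP_Card actors by lerping them to target transforms.
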(event `self.ReceiveBeginPlay`
  (bind _asbp_pawn (cast `/Game/Blueprints/BP_Pawn` (`Controller.K2_GetPawn` (`GameplayStatics.GetPlayerController` 0))))
  (set `self.LocalPawn` _asbp_pawn))

(event `OnTurnEnded`
  (`self.HighlightAllCards` false)
  (`/Game/Blueprints/BP_Pawn.SwitchView` (`self.LocalPawn`) "NewEnumerator0"))

(event `OnAbilityActivated`
  (params (Player :type "Controller Object Reference") (Ability :type "ECardAbility Enum" :default "None"))
  (switch `ECardAbility` Ability
    (:`RevealOpponentOne`
      (`/Game/Blueprints/BP_Pawn.SwitchView` (`self.LocalPawn`) "NewEnumerator1" :!label _label)
      (`self.HighlightAllOpponentCards` true :!label _label_2)
      (`self.HighlightOwnedCards` true))
    (:`RevealSelfOne`
      (`self.HighlightOwnedCards` true :!label _label_3))
    (:`SwapOneNoReveal`
      (`/Game/Blueprints/BP_Pawn.SwitchView` (`self.LocalPawn`) "NewEnumerator2")
      (goto _label_2))
    (:`RevealOneEachOpponent`
      (goto _label))
    (:`DiscardOneSelf`
      (goto _label_3))))

(event `HighlightAllCards`
  (params (`On?` :type Boolean))
  (bind _outactors (`GameplayStatics.GetAllActorsOfClass` "/Game/Blueprints/BP_Card.BP_Card_C"))
  (for _array_element _outactors
    (message `/Game/Blueprints/BPI_Interaction.Highlight` _array_element `On?`)))

(event `HighlightOwnedCards`
  (params (`On?` :type Boolean))
  (bind _outactors (`GameplayStatics.GetAllActorsOfClass` "/Game/Blueprints/BP_Card.BP_Card_C"))
  (for _array_element _outactors
    (if (== (`self.GetOwner` _array_element) (`GameplayStatics.GetPlayerController` 0))
      (message `/Game/Blueprints/BPI_Interaction.Highlight` _array_element `On?`))))

(event `HighlightAllOpponentCards`
  (params (`On?` :type Boolean))
  (bind _outactors (`GameplayStatics.GetAllActorsOfClass` "/Game/Blueprints/BP_Card.BP_Card_C"))
  (for _array_element _outactors
    (if (!= (`self.GetOwner` _array_element) (`GameplayStatics.GetPlayerController` 0))
      (message `/Game/Blueprints/BPI_Interaction.Highlight` _array_element `On?`))))

(event `HighlightCards`
  (params (Card :type "Array of /Game/Blueprints/BP_Card Object Reference") (`On?` :type Boolean))
  (for _array_element Card
    (message `/Game/Blueprints/BPI_Interaction.Highlight` _array_element `On?`)))

(event `OnCardDestroyed`
  (params (Card :type "/Game/Blueprints/BP_Card Object Reference") (EndTransform :type "Transform Structure"))
  (`/Game/Blueprints/BP_Card.LerpCardTo` Card EndTransform true))

(event `OnCardSwapped`
  (params (`Keep Card` :type "Card Object Reference") (`Discard Card` :type "Card Object Reference"))
  (bind _asbp_card (cast `/Game/Blueprints/BP_Card` `Keep Card`))
  (`/Game/Blueprints/BP_Card.LerpCardTo` _asbp_card (`self.GetTransform` `Discard Card`) false))

(event `CLIENT HighlightOwnedCards`
  (params (`On?` :type Boolean))
  (`self.HighlightOwnedCards` `On?`))

(event `CLIENT OpponentCardSwap`
  (params (`Card 1` :type "/Game/Blueprints/BP_Card Object Reference") (`Card 2` :type "/Game/Blueprints/BP_Card Object Reference"))
  (bind _output_get (set `self.Temp` (`self.GetTransform` `Card 1`)))
  (`/Game/Blueprints/BP_Card.LerpCardTo` `Card 2` _output_get false)
  (`/Game/Blueprints/BP_Card.LerpCardTo` `Card 1` (`self.GetTransform` `Card 2`) false))

(fn `UserConstructionScript`)