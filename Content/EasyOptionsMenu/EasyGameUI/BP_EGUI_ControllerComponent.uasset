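; Player controller component for the EGUI menu system that handles UI navigation input, widget focus and cursor visibility.
; It adds a base Enhanced Input mapping context and forwards navigation, apply, reset and any-key presses to registered listener widgets.
; Gamepad or keyboard input hides and parks the cursor and restores lost focus, while mouse movement shows it again.
; It also shows a reusable alert banner, handing focus to it and back to the underlying widget.
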(event `self.ReceiveBeginPlay`
  ;[0.4583 1 1 1 40] Init
  (bind _asplayer_controller (cast `PlayerController` (`self.GetOwner`))
    (:`then`
      (set `self.PlayerController` _asplayer_controller)
      (`self.AddBaseInputMappingContext`))
    (:`CastFailed`
      (`KismetSystemLibrary.PrintString` "ERROR! The EGUI Controller Component has not been added to a player controller.  \nPlease make sure to add it to your Player Controller (not Player Character) or use the provided one.  \nCheck out the documentation for more informations." true true (struct :`R` 1.0 :`A` 1.0) 100.0))))

(event `EnhancedInput|/Game/EasyOptionsMenu/EasyGameUI/UINavigation/IA_HeaderNav`
  (params (ActionValue :type "Float (double-precision)") (ElapsedSeconds :type "Float (double-precision)") (TriggeredSeconds :type "Float (double-precision)") (InputAction :type "InputAction Object Reference" :default "/Game/EasyOptionsMenu/EasyGameUI/UINavigation/IA_HeaderNav.IA_HeaderNav"))
  ;[1 0.3176 0.4579 1 40] Handle UI Navigation Events
  (:`Triggered`
    (`/Engine/EditorBlueprintResources/StandardMacros.DoOnce` false :!label _label
      (:`Completed`
        (`/Game/EasyOptionsMenu/EasyGameUI/BFL_EasyFunctionUtilities.InputTriggered` (`self.InputListeningWidgets`) self "NewEnumerator0" (`KismetStringLibrary.Conv_DoubleToString` ActionValue)))))
  (:`Completed`
    (goto _label :!via `Reset`)))

(event `EnhancedInput|/Game/EasyOptionsMenu/EasyGameUI/UINavigation/IA_NavBack`
  (params (ActionValue :type Boolean) (ElapsedSeconds :type "Float (double-precision)") (TriggeredSeconds :type "Float (double-precision)") (InputAction :type "InputAction Object Reference" :default "/Game/EasyOptionsMenu/EasyGameUI/UINavigation/IA_NavBack.IA_NavBack"))
  ;[1 0.3176 0.4579 1 40] Handle UI Navigation Events
  (:`Started`
    (`/Game/EasyOptionsMenu/EasyGameUI/BFL_EasyFunctionUtilities.InputTriggered` (`self.InputListeningWidgets`) self "NewEnumerator1" (`KismetStringLibrary.Conv_BoolToString` ActionValue))))

(event `Key|AnyKey` :consume false :paused true :overrideparent false
  (params (Key :type "Key Structure"))
  ;[1 0.3176 0.4579 1 40] Handle UI Navigation Events
  (:`Pressed`
    (bind _output (`/Game/EasyOptionsMenu/EasyGameUI/BML_EasyMacroUtilities.GetAllValidListeningWidgets` (`self.InputListeningWidgets`) self)
      (:`Is Valid`
        (message `/Game/EasyOptionsMenu/EasyGameUI/UINavigation/BPI_InputNavigation.AnyKeyPressed` _output Key)))))

(event `EnhancedInput|/Game/EasyOptionsMenu/EasyGameUI/UINavigation/IA_NavForward`
  (params (ActionValue :type Boolean) (ElapsedSeconds :type "Float (double-precision)") (TriggeredSeconds :type "Float (double-precision)") (InputAction :type "InputAction Object Reference" :default "/Game/EasyOptionsMenu/EasyGameUI/UINavigation/IA_NavForward.IA_NavForward"))
  ;[1 0.3176 0.4579 1 40] Handle UI Navigation Events
  (:`Started`
    (`/Game/EasyOptionsMenu/EasyGameUI/BFL_EasyFunctionUtilities.InputTriggered` (`self.InputListeningWidgets`) self "NewEnumerator2" (`KismetStringLibrary.Conv_BoolToString` ActionValue))))

(event `EnhancedInput|/Game/EasyOptionsMenu/EasyGameUI/UINavigation/IA_ApplySettings`
  (params (ActionValue :type Boolean) (ElapsedSeconds :type "Float (double-precision)") (TriggeredSeconds :type "Float (double-precision)") (InputAction :type "InputAction Object Reference" :default "/Game/EasyOptionsMenu/EasyGameUI/UINavigation/IA_ApplySettings.IA_ApplySettings"))
  ;[1 0.3176 0.4579 1 40] Handle UI Navigation Events
  (:`Started`
    (`/Game/EasyOptionsMenu/EasyGameUI/BFL_EasyFunctionUtilities.InputTriggered` (`self.InputListeningWidgets`) self "NewEnumerator3" (`KismetStringLibrary.Conv_BoolToString` ActionValue))))

(event `/Game/EasyOptionsMenu/EasyGameUI/UINavigation/BPI_InputNavigation.RegisterInputListener`
  (params (Widget :type "UserWidget Soft Object Reference"))
  ;[1 0.3176 0.4579 1 40] Handle UI Navigation Events
  ;;[0.6358 1 0.4314 1 30] Handle Widget Registration
  (`/Game/EasyOptionsMenu/EasyGameUI/BFL_EasyFunctionUtilities.RegisterInputListenerFromArray` (`self.InputListeningWidgets`) Widget (`self.PlayerController`)))

(event `/Game/EasyOptionsMenu/EasyGameUI/UINavigation/BPI_InputNavigation.UnregisterInputListener`
  (params (Widget :type "UserWidget Soft Object Reference"))
  ;[1 0.3176 0.4579 1 40] Handle UI Navigation Events
  ;;[0.6358 1 0.4314 1 30] Handle Widget Registration
  (`/Game/EasyOptionsMenu/EasyGameUI/BFL_EasyFunctionUtilities.UnregisterInputListenerFromArray` (`self.InputListeningWidgets`) Widget (`self.PlayerController`)))

(event `EnhancedInput|/Game/EasyOptionsMenu/EasyGameUI/UINavigation/IA_ResetSettings`
  (params (ActionValue :type Boolean) (ElapsedSeconds :type "Float (double-precision)") (TriggeredSeconds :type "Float (double-precision)") (InputAction :type "InputAction Object Reference" :default "/Game/EasyOptionsMenu/EasyGameUI/UINavigation/IA_ResetSettings.IA_ResetSettings"))
  ;[1 0.3176 0.4579 1 40] Handle UI Navigation Events
  (:`Started`
    (`/Game/EasyOptionsMenu/EasyGameUI/BFL_EasyFunctionUtilities.InputTriggered` (`self.InputListeningWidgets`) self "NewEnumerator4" (`KismetStringLibrary.Conv_BoolToString` ActionValue))))

(fn `AddBaseInputMappingContext`
  (`EnhancedInputSubsystemInterface.AddMappingContext` (pcsubsystem `EnhancedInputLocalPlayerSubsystem` (`self.PlayerController`)) (`self.BaseInputMappingContext`) 0 (struct)))

(fn `HandleCursorVisibility`
  (params (WidgetReference :type "Widget Object Reference") (`ShouldHideMouseCursor?` :type Boolean))
  (bind _playercontroller (`self.PlayerController`))
  (bind _playercontroller_2 (`self.PlayerController`))
  (bind _widgetreference (`local.WidgetReference`))
  (bind (_last_mouse_position_x _last_mouse_position_y) (`KismetMathLibrary.BreakVector2D` (`self.Last Mouse Position`)))
  (bind (_locationx _locationy) (`PlayerController.GetMousePosition` _playercontroller_2))
  (bind (_locationx_2 _locationy_2) (`PlayerController.GetMousePosition` (`self.PlayerController`)))
  (if `ShouldHideMouseCursor?`
    (if (`PlayerController.bShowMouseCursor` _playercontroller_2)
      (if (and (!= _locationx_2 20.0) (!= _locationy_2 20.0))
        (set `self.Last Mouse Position` (`KismetMathLibrary.MakeVector2D` _locationx_2 _locationy_2)))
      (set `PlayerController.bShowMouseCursor` false _playercontroller)
      (`PlayerController.SetMouseLocation` _playercontroller 20 20)
      (`Widget.SetCursor` _widgetreference "None"))
    (elif (and (not (`PlayerController.bShowMouseCursor` _playercontroller_2)) (!= _locationx 20.0) (!= _locationy 20.0))
      (set `PlayerController.bShowMouseCursor` true _playercontroller)
      (`PlayerController.SetMouseLocation` _playercontroller (`KismetMathLibrary.FTrunc` _last_mouse_position_x) (`KismetMathLibrary.FTrunc` _last_mouse_position_y))
      (`Widget.SetCursor` _widgetreference "Default"))))

(fn `HandleFocusLoss`
  (params (Key :type "Key Structure (by ref)") (WidgetReference :type "Widget Object Reference") (ElementToRefocus :type "Widget Object Reference"))
  (bind _widgetreference (`local.WidgetReference`))
  (if (or (`KismetInputLibrary.Key_IsGamepadKey` Key) (`KismetInputLibrary.Key_IsKeyboardKey` Key))
    (`self.HandleCursorVisibility` _widgetreference true)
    (if (`self.LostFocus?`)
      (bind _elementtorefocus (`local.ElementToRefocus`)
        (:`then`
          (`Widget.SetKeyboardFocus` _elementtorefocus))
        (:`else`
          _))
      (set `self.LostFocus?` false))
    (else
      (`self.HandleCursorVisibility` _widgetreference)
      (set `self.LostFocus?` true))))

(fn `HandleMouseMovementDetection`
  (params (MouseEvent :type "PointerEvent Structure (by ref)") (WidgetReference :type "Widget Object Reference"))
  (returns (ReturnValue :type "EventReply Structure"))
  (if (> (`KismetMathLibrary.VSize2D` (`KismetInputLibrary.PointerEvent_GetCursorDelta` MouseEvent)) 0.0)
    (`self.HandleCursorVisibility` (`local.WidgetReference`))
    (return (`WidgetBlueprintLibrary.Unhandled`))))

(fn `InitializeFocusHandling`
  (params (WidgetReference :type "UserWidget Object Reference") (InitialElementToFocus :type "Widget Object Reference") (`RegisterInputListener?` :type Boolean :default true) (`SetInputModeGameAndUI?` :type Boolean :default true))
  (set `PlayerController.bShowMouseCursor` true (`self.PlayerController`))
  (`self.HandleCursorVisibility` (`local.WidgetReference`) true)
  (set `self.LostFocus?` false)
  (if (`local.RegisterInputListener?`)
    (`self.RegisterInputListener` (`|ConvertAsset` (`local.WidgetReference`))))
  (if (`local.SetInputModeGameAndUI?`)
    (`WidgetBlueprintLibrary.SetInputMode_GameAndUIEx` (`self.PlayerController`) (`local.WidgetReference`) "DoNotLock" false true))
  (bind _initialelementtofocus (`local.InitialElementToFocus`)
    (:`then`
      (`Widget.SetKeyboardFocus` _initialelementtofocus))
    (:`else`)))

(fn `RemoveBaseInputMappingContext`
  (`EnhancedInputSubsystemInterface.RemoveMappingContext` (pcsubsystem `EnhancedInputLocalPlayerSubsystem` (`self.PlayerController`)) (`self.BaseInputMappingContext`) (struct)))

(fn `ResetFocusFromAlertBanner`
  (params (UnderlyingWidget :type "UserWidget Object Reference") (ElementToRefocus :type "Widget Object Reference"))
  (bind _alertbannerreference (`self.AlertBannerReference`))
  (`Widget.SetVisibility` UnderlyingWidget "SelfHitTestInvisible")
  (`self.InitializeFocusHandling` (`local.UnderlyingWidget`) (`local.ElementToRefocus`) true false)
  (`self.UnregisterInputListener` (`|ConvertAsset` _alertbannerreference))
  (clear `/Game/EasyOptionsMenu/EasyGameUI/CommonWidgets/WBP_EGUI_CommonAlertBanner.ActionRequested` _alertbannerreference)
  (`Widget.RemoveFromParent` _alertbannerreference))

(fn `SetupAlertBanner`
  (params (UnderlyingWidget :type "UserWidget Object Reference") (`Action Description` :type Text) (`Options Buttons` :type "Array of Text") (ButtonsSizeRule :type "ESlateSizeRule Enum" :default "Fill") (DelayBeforeAutomaticAction :type Integer) (ActionToExecuteAfterDelay :type Integer))
  (returns (BannerWidget :type "/Game/EasyOptionsMenu/EasyGameUI/CommonWidgets/WBP_EGUI_CommonAlertBanner Object Reference"))
  (bind _underlyingwidget (`local.UnderlyingWidget`))
  (bind _alertbannerreference (`self.AlertBannerReference`))
  (bind _alertbannerreference_2 (`self.AlertBannerReference`)
    (:`then`
      (if (not (`Widget.IsInViewport` _alertbannerreference_2))
        (`UserWidget.AddToViewport` _alertbannerreference 999 :!label _label)))
    (:`else`
      (bind _returnvalue (`|CreateWidget` "/Game/EasyOptionsMenu/EasyGameUI/CommonWidgets/WBP_EGUI_CommonAlertBanner.WBP_EGUI_CommonAlertBanner_C"))
      (set `self.AlertBannerReference` _returnvalue)
      (goto _label)))
  (set `/Game/EasyOptionsMenu/EasyGameUI/CommonWidgets/WBP_EGUI_CommonAlertBanner.ButtonsSizeRule` (`local.ButtonsSizeRule`) _alertbannerreference)
  (`/Game/EasyOptionsMenu/EasyGameUI/CommonWidgets/WBP_EGUI_CommonAlertBanner.SetupWidget` _alertbannerreference self (`local.Action Description`) (`local.Options Buttons`) (`local.DelayBeforeAutomaticAction`) (`local.ActionToExecuteAfterDelay`))
  (`self.InitializeFocusHandling` (`self.AlertBannerReference`) null true false)
  (`Widget.SetVisibility` _underlyingwidget "HitTestInvisible")
  (`self.UnregisterInputListener` (`|ConvertAsset` _underlyingwidget))
  (return (`self.AlertBannerReference`)))